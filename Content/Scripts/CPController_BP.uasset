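; Checkpoint controller that tracks which CheckPoint_BP actors have been crossed in a race.
; On BeginPlay it gathers the checkpoints into AllCheckPoints and sizes a matching CheckPointCrossed flag array.
; SortArray is meant to order them, but its step parsing numbers from display-name suffixes is disconnected.
; HandleRace checks whether all flags are set, then clears RaceComplete and sets the first flag true.
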(event EventBeginPlay
  (CallFunction|InitializeAllCheckpointActors)
  (Development|PrintString (Utilities|String|Append "Checkpoint system initialized with " (Utilities|String|ToString(Integer) (Utilities|Array|Length (Variables|Default|GetAll_CheckPoints))) "/" (Utilities|String|ToString(Integer) (Utilities|Array|Length (Variables|Default|GetCheckPointCrossed))) " checkpoints")))

(event Collision|EventActorBeginOverlap
  (params (OtherActor :type Actor%20Object%20Reference)))

(event EventTick
  (params (DeltaSeconds :type Float%20%28single-precision%29)))

(fn ConstructionScript)

(fn InitializeAllCheckpointActors
  (bind _outactors (Actor|GetAllActorsOfClass "/Game/Scripts/CheckPoint_BP.CheckPoint_BP_C"))
  (bind _newparam (CallFunction|SortArray _outactors))
  (bind _output_get (Variables|Default|SetAll_CheckPoints _newparam))
  (for _array_element _output_get
    (Development|PrintString (Utilities|GetDisplayName _array_element) false true "(R=1.000000,G=0.000000,B=0.050402,A=1.000000)"))
  (for (_ _array_index) _output_get
    (Utilities|Array|SetArrayElem (Variables|Default|GetCheckPointCrossed) _array_index false true)))

(fn PrintAllCheckpoints
  (for (_array_element _array_index) (Variables|Default|GetCheckPointCrossed)
    (Variables|Default|SetOutputString (Utilities|String|MakeLiteralString (Utilities|String|Append (Variables|Default|GetOutputString) "/ Checkpoint  " (Utilities|String|ToString(Integer) _array_index) " is " (Utilities|String|ToString(Boolean) _array_element) "/"))))
  (Development|PrintString (Variables|Default|GetOutputString)))

(fn HandleRace
  (LocalVariables|SetRaceComplete true)
  (for _array_element (Variables|Default|GetCheckPointCrossed)
    (if (not _array_element)
      (LocalVariables|SetRaceComplete false)))
  (if (LocalVariables|GetRaceComplete)
    (for _array_element_2 (Variables|Default|GetCheckPointCrossed)
      (LocalVariables|SetRaceComplete false))
    (Utilities|Array|SetArrayElem (Variables|Default|GetCheckPointCrossed) 0 true)))

(fn SortArray
  (params (Input :type Array%20of%20Check%20Point%20BP%20Object%20References))
  (bind _sortingints (LocalVariables|GetSortingInts))
  (bind _output (LocalVariables|GetOutput))
  (for (_array_element _array_index) Input
    (Utilities|Array|AppendArray (LocalVariables|GetOutput) Input)
    (for (_ _array_index_2) _sortingints
      (Utilities|Array|SetArrayElem _output _array_index_2 (Utilities|Array|Get(acopy) (Variables|Default|GetAll_CheckPoints) (Utilities|Array|FindItem _sortingints _array_index_2))))
    (return _output)))