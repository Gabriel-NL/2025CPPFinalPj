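; Checkpoint actor that records when any actor overlaps it.
; On BeginPlay it caches the first CPController_BP in the level, then on overlap finds its own index in that controller's AllCheckPoints and flags the matching CheckPointCrossed entry.
; Each overlap also loops through every checkpoint, printing its crossed state and playing a ding at the world origin per iteration.
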(event EventBeginPlay
  (CallFunction|ConnecttoController))

(event Collision|EventActorBeginOverlap
  (params (OtherActor :type Actor%20Object%20Reference))
  (bind _cp_controller_var (Variables|Default|GetCP_controller_var))
  (CallFunction|CollidedwithCheckpoint)
  (for (_ _array_index) (Variables|/Game/Scripts/CPController_BP.CPController_BP_C|GetAll_CheckPoints _cp_controller_var)
    (Development|PrintString (Utilities|String|Append "Checkpoint:" (Utilities|String|ToString(Integer) _array_index) "Value: " (Utilities|String|ToString(Boolean) (Utilities|Array|Get(acopy) (Variables|/Game/Scripts/CPController_BP.CPController_BP_C|GetCheckPointCrossed _cp_controller_var) _array_index))))
    (Audio|PlaySoundatLocation "/Game/Audio/Ding_Cue.Ding_Cue" "0, 0, 0" "0, 0, 0" 1.0 1.0 0.0 0 0 0)))

(event EventTick
  (params (DeltaSeconds :type Float%20%28single-precision%29)))

(fn ConstructionScript)

(fn ConnecttoController
  (bind _outactors (Actor|GetAllActorsOfClass "/Game/Scripts/CPController_BP.CPController_BP_C"))
  (Variables|Default|SetCP_controller_var (Utilities|Array|Get(acopy) _outactors)))

(fn CollidedwithCheckpoint
  (bind _cp_controller_var (Variables|Default|GetCP_controller_var))
  (Utilities|IsValid _cp_controller_var
    (:Is%20Valid
      (Utilities|Array|SetArrayElem (Variables|/Game/Scripts/CPController_BP.CPController_BP_C|GetCheckPointCrossed (Variables|Default|GetCP_controller_var)) (Utilities|Array|FindItem (Variables|/Game/Scripts/CPController_BP.CPController_BP_C|GetAll_CheckPoints _cp_controller_var) self) true))
    (:Is%20Not%20Valid
      (Development|PrintString "CP_controller not found"))))